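; Interactive door actor that swings open and closed when the player presses E nearby.
; Overlapping Trigger_Box enables input for player controller 0, and leaving it disables input, without checking which actor overlaps.
; Each press flips DoorStatus and plays or reverses the Door_Rotation timeline, whose DoorRot track sets the yaw of the whole actor's relative rotation.
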(event `self.Trigger_Box.OnComponentBeginOverlap`
  (params (OtherActor :type "Actor Object Reference") (OtherComp :type "PrimitiveComponent Object Reference") (OtherBodyIndex :type Integer) (bFromSweep :type Boolean) (SweepResult :type "EngineTypes.HitResult Structure (by ref)"))
  (`self.EnableInput` (`GameplayStatics.GetPlayerController` 0)))

(event `Key|E`
  (:`Pressed`
    (if (`self.Door_Status`)
      (set `self.Door_Status` false)
      (bind (_direction _doorrot) (`Timeline|Door_Rotation` :!label _label)
        (:`Update`
          (`self.K2_SetActorRelativeRotation` (`KismetMathLibrary.MakeRot` 0.0 _doorrot))))
      (else
        (set `self.Door_Status` true)
        (goto _label :!via `Reverse`)))))

(event `self.Trigger_Box.OnComponentEndOverlap`
  (params (OtherActor :type "Actor Object Reference") (OtherComp :type "PrimitiveComponent Object Reference") (OtherBodyIndex :type Integer))
  (`self.DisableInput` (`GameplayStatics.GetPlayerController` 0)))

(fn `UserConstructionScript`)